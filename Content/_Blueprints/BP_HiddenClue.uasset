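; BP_HiddenClue is a clue actor whose visibility can be toggled through its Show and Hide functions.
; On BeginPlay it spawns a BP_HiddenClueManager at the world origin if none exists, so placing a clue guarantees a manager.
; Show and Hide set visibility on its two static meshes and on the first static mesh component found in each attached actor.
; A mesh rotation node remains in the graph but is never run.
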(event `self.ReceiveBeginPlay`
  (bind _returnvalue (`GameplayStatics.GetActorOfClass` "/Game/_Blueprints/BP_HiddenClueManager.BP_HiddenClueManager_C"))
  (if (not (`KismetSystemLibrary.IsValid` _returnvalue))
    (`|SpawnActorFromClass` "/Game/_Blueprints/BP_HiddenClueManager.BP_HiddenClueManager_C" (`KismetMathLibrary.MakeTransform` (0.0 0.0 0.0)) "AlwaysSpawn" "OverrideRootScale" null null)))

(event `self.ReceiveTick`
  (params (DeltaSeconds :type "Float (single-precision)")))

(fn `Hide`
  (`SceneComponent.SetVisibility` (`self.StaticMesh`) false true)
  (`SceneComponent.SetVisibility` (`self.StaticMesh1`) false true)
  (for _array_element (`self.GetAttachedActors` self true)
    (bind _returnvalue (`self.GetComponentByClass` _array_element "/Script/Engine.StaticMeshComponent"))
    (if (`KismetSystemLibrary.IsValid` _returnvalue)
      (`SceneComponent.SetVisibility` _returnvalue false true))))

(fn `Show`
  (`SceneComponent.SetVisibility` (`self.StaticMesh`) true true)
  (`SceneComponent.SetVisibility` (`self.StaticMesh1`) true true)
  (for _array_element (`self.GetAttachedActors` self true)
    (bind _returnvalue (`self.GetComponentByClass` _array_element "/Script/Engine.StaticMeshComponent"))
    (if (`KismetSystemLibrary.IsValid` _returnvalue)
      (`SceneComponent.SetVisibility` _returnvalue true true))))

(fn `UserConstructionScript`)