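; Manager actor that toggles the visibility of all BP_HiddenClue actors in the level.
; On BeginPlay it enables input from player controller 0 and runs the toggle once to apply a starting state.
; Pressing the 1 key flips the Hidden flag, then calls HideAll or ShowAll.
; Both functions gather every clue with GetAllActorsOfClass on each call and invoke its Hide or Show.
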(event `Key|One`
  (params (Key :type "Key Structure"))
  (:`Pressed`
    (bind _output_get (set `self.Hidden` (not (`self.Hidden`)) :!label _label))
    (if _output_get
      (`self.HideAll`)
      (else
        (`self.ShowAll`)))))

(event `self.ReceiveBeginPlay`
  (`self.EnableInput` (`GameplayStatics.GetPlayerController` 0))
  (goto _label))

(fn `HideAll`
  (bind _outactors (`GameplayStatics.GetAllActorsOfClass` "/Game/_Blueprints/BP_HiddenClue.BP_HiddenClue_C"))
  (for _array_element _outactors
    (`/Game/_Blueprints/BP_HiddenClue.Hide` _array_element)))

(fn `ShowAll`
  (bind _outactors (`GameplayStatics.GetAllActorsOfClass` "/Game/_Blueprints/BP_HiddenClue.BP_HiddenClue_C"))
  (for _array_element _outactors
    (`/Game/_Blueprints/BP_HiddenClue.Show` _array_element)))

(fn `UserConstructionScript`)